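; Puzzle win trigger that completes the level once a BP_PuzzlePawn stays overlapped for half a second.
; Tick accumulates overlap time through a resettable DoOnce, and leaving the trigger resets both.
; On a win it disables player input, waits a second, destroys or re-materials tagged actors, and stops pawn rotation.
; It then plays a level sequence whose finish event opens the configured next level.
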(event `LoadNextLevel`
  (`GameplayStatics.OpenLevel` (`self.LevelToLoad`)))

(event `self.ReceiveBeginPlay`
  (add `MovieSceneSequencePlayer.OnFinished` (`LevelSequenceActor.SequencePlayer` (`self.LevelSequence`)) (delegate `LoadNextLevel`)))

(event `self.ReceiveActorBeginOverlap`
  (params (OtherActor :type "Actor Object Reference"))
  (bind _asbp_puzzle_pawn (cast `/Game/Blueprints/BP_PuzzlePawn` OtherActor))
  (set `self.Overlapping Actor` _asbp_puzzle_pawn)
  (set `self.startcountingB` true))

(event `self.ReceiveTick`
  (params (DeltaSeconds :type "Float (single-precision)"))
  (bind _time (`self.Time`))
  (if (`self.startcountingB`)
    (set `self.Time` (+ _time DeltaSeconds))
    (if (>= _time 0.5)
      (`/Engine/EditorBlueprintResources/StandardMacros.DoOnce` false :!label _label
        (:`Completed`
          (`self.DisableInput` (`GameplayStatics.GetPlayerPawn` 0) (`GameplayStatics.GetPlayerController` 0))
          (`KismetSystemLibrary.Delay` 1.0)
          (bind _outactors (`GameplayStatics.GetAllActorsWithTag` "DestroyOnWin"))
          (for _array_element _outactors
            (`self.K2_DestroyActor` _array_element))
          (bind _outactors_2 (`GameplayStatics.GetAllActorsWithTag` "GlowOnWin"))
          (for _array_element_2 _outactors_2
            (bind _asstatic_mesh_actor (cast `StaticMeshActor` _array_element_2))
            (`PrimitiveComponent.SetMaterial` (`StaticMeshActor.StaticMeshComponent` _asstatic_mesh_actor) 0 "/Game/Environments/Three/Big_Strip.Big_Strip"))
          (bind _aspuzzle_pawn (cast `PuzzlePawn` (`GameplayStatics.GetPlayerPawn` 0)))
          (set `PuzzlePawn.CanRotate` false _aspuzzle_pawn)
          (`MovieSceneSequencePlayer.Play` (`LevelSequenceActor.SequencePlayer` (`self.LevelSequence`))))))))

(event `self.ReceiveActorEndOverlap`
  (params (OtherActor :type "Actor Object Reference"))
  (if (== OtherActor (`self.Overlapping Actor`))
    (set `self.Time` 0.0)
    (set `self.startcountingB` false)
    (set `self.Overlapping Actor` null)
    (goto _label :!via `Reset`)))

(fn `UserConstructionScript`)